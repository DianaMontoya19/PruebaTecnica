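; Enemy AI character that spawns with a sword, patrols random points, and chases and attacks the player.
; Capsule overlap switches between patrolling and AIMoveTo pursuit with a looping attack timer.
; Attacks set IA_Enemy animation flags by attack state and briefly enable DamageRange collision to deal damage.
; GetDamage triggers death at zero life, while Tick updates the life bar and halts fighting when the player's StoppGame is set.
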(event `self.ReceiveBeginPlay`
  (`|ExecutionSequence`
    (:`then_0`
      (`PrimitiveComponent.SetCollisionEnabled` (`self.DamageRange`) "NoCollision"))
    (:`then_1`
      (bind _returnvalue (`|SpawnActorFromClass` "/Game/Blueprints/BP_SwordEnemy.BP_SwordEnemy_C" (`SceneComponent.GetSocketTransform` (`self.Mesh`) "b_MF_Weapon_R_Socket" "RTS_World") "Undefined" "MultiplyWithRoot" null null))
      (bind _output_get (set `self.TrollSword` _returnvalue))
      (`self.K2_AttachToComponent` _output_get (`self.Mesh`) "b_MF_Weapon_R_Socket" "SnapToTarget" "SnapToTarget" "SnapToTarget" true))
    (:`then_2`
      (if (not (`self.PlayerDetected`))
        (`self.StartPatrol`)))))

(event `self.PawnSensing.OnSeePawn`
  (params (Pawn :type "Pawn Object Reference")))

(event `FollowPlayer`
  (if (`self.PlayerDetected`)
    (`|AIMoveTo` self (0.0 0.0 0.0) (`GameplayStatics.GetPlayerCharacter` 0))))

(event `self.Capsule.OnComponentBeginOverlap`
  (params (OverlappedComponent :type "PrimitiveComponent Object Reference") (OtherActor :type "Actor Object Reference") (OtherComp :type "PrimitiveComponent Object Reference") (OtherBodyIndex :type Integer) (bFromSweep :type Boolean) (SweepResult :type "HitResult Structure (by ref)"))
  (cast `/Game/ThirdPerson/Blueprints/BP_ThirdPersonCharacter` OtherActor)
  (set `self.RangeOfAttack` true)
  (set `self.PlayerDetected` true)
  (`self.StartAttackLoop`)
  (`self.StopPatrol`)
  (`self.FollowPlayer`))

(event `self.Capsule.OnComponentEndOverlap`
  (params (OverlappedComponent :type "PrimitiveComponent Object Reference") (OtherActor :type "Actor Object Reference") (OtherComp :type "PrimitiveComponent Object Reference") (OtherBodyIndex :type Integer))
  (cast `/Game/ThirdPerson/Blueprints/BP_ThirdPersonCharacter` OtherActor)
  (set `self.RangeOfAttack` false)
  (set `self.PlayerDetected` false)
  (`self.StopAttackLoop`)
  (`self.StartPatrol`))

(event `StopAttackLoop`
  (`KismetSystemLibrary.K2_ClearAndInvalidateTimerHandle` (`self.LoopTimerAttack`))
  (`KismetSystemLibrary.PrintString` "No mas ataque"))

(event `StartAttackLoop`
  (if (not (`KismetSystemLibrary.K2_IsTimerActiveHandle` (struct)))
    (bind _returnvalue (`KismetSystemLibrary.K2_SetTimerDelegate` (delegate `PerfomAttack`) (`self.AttackCoolDown`) true))
    (set `self.LoopTimerAttack` _returnvalue)))

(event `PerfomAttack`
  (if (`self.RangeOfAttack`)
    (if (`self.CanAttack`)
      (bind _asia_enemy (cast `/Game/IA_Animations/IA_Enemy` (`SkeletalMeshComponent.GetAnimInstance` (`self.Mesh`))))
      (`self.StatesOfEnemy` _asia_enemy)
      (set `self.CanAttack` false)
      (`KismetSystemLibrary.Delay` (`self.AttackCoolDown`))
      (set `/Game/IA_Animations/IA_Enemy.NoCollision` false _asia_enemy)
      (`PrimitiveComponent.SetCollisionEnabled` (`self.DamageRange`) "QueryAndPhysics")
      (`KismetSystemLibrary.PrintString` "Colision activa")
      (`KismetSystemLibrary.Delay` 1.0)
      (set `/Game/IA_Animations/IA_Enemy.NoCollision` true _asia_enemy)
      (`PrimitiveComponent.SetCollisionEnabled` (`self.DamageRange`) "NoCollision")
      (`KismetSystemLibrary.PrintString` "No collision")
      (set `self.CanAttack` true))))

(event `StatesOfEnemy`
  (params (Enemy :type "/Game/IA_Animations/IA_Enemy Object Reference"))
  (bind _output_get (set `/Game/IA_Animations/IA_Enemy.CurrentStateEnemy` (`self.States`) Enemy))
  (switch `/Game/Blueprints/EStatesEnemy` _output_get
    (:`NewEnumerator0`
      (set `/Game/IA_Animations/IA_Enemy.ExoAttack` true Enemy))
    (:`NewEnumerator1`
      (set `/Game/IA_Animations/IA_Enemy.Attack` true Enemy))
    (:`NewEnumerator2`
      (set `/Game/IA_Animations/IA_Enemy.FinalAttack` true Enemy))))

(event `NoFightMore`
  (`MovementComponent.StopMovementImmediately` (`self.CharacterMovement`))
  (bind _asia_enemy (cast `/Game/IA_Animations/IA_Enemy` (`SkeletalMeshComponent.GetAnimInstance` (`self.Mesh`))))
  (bind _output_get (set `/Game/IA_Animations/IA_Enemy.CurrentStateEnemy` (`self.States`) _asia_enemy))
  (switch `/Game/Blueprints/EStatesEnemy` _output_get
    (:`NewEnumerator0`
      (set `/Game/IA_Animations/IA_Enemy.ExoAttack` false _asia_enemy))
    (:`NewEnumerator1`
      (set `/Game/IA_Animations/IA_Enemy.Attack` false _asia_enemy))
    (:`NewEnumerator2`
      (set `/Game/IA_Animations/IA_Enemy.FinalAttack` false _asia_enemy))))

(event `StopPatrol`
  (if (`self.IsPatrol`)
    (set `self.IsPatrol` false)
    (`MovementComponent.StopMovementImmediately` (`self.CharacterMovement`))
    (`self.FollowPlayer`)
    (`KismetSystemLibrary.PrintString` "StopPatrol")))

(event `StartPatrol`
  (if (not (`self.IsPatrol`))
    (set `self.IsPatrol` true)
    (`MovementComponent.StopMovementImmediately` (`self.CharacterMovement`))
    (`self.MoveToNextPatrol`)
    (`KismetSystemLibrary.PrintString` "StartPatrol")))

(event `self.DamageRange.OnComponentBeginOverlap`
  (params (OverlappedComponent :type "PrimitiveComponent Object Reference") (OtherActor :type "Actor Object Reference") (OtherComp :type "PrimitiveComponent Object Reference") (OtherBodyIndex :type Integer) (bFromSweep :type Boolean) (SweepResult :type "HitResult Structure (by ref)"))
  (bind _asbp_third_person_character (cast `/Game/ThirdPerson/Blueprints/BP_ThirdPersonCharacter` OtherActor))
  (`/Game/ThirdPerson/Blueprints/BP_ThirdPersonCharacter.GetDamage` _asbp_third_person_character 10.0))

(event `MoveToNextPatrol`
  (if (`self.IsPatrol`)
    (if (> (`KismetArrayLibrary.Array_Length` (`self.PatrolPawn`)) 0)
      (bind _output_get (set `self.CurrentIndexPatrol` (`KismetMathLibrary.RandomIntegerInRange` 0 (`KismetArrayLibrary.Array_Length` (`self.PatrolPawn`)))))
      (`|AIMoveTo` self (`|GetArrayItem` (`self.PatrolPawn`) _output_get) null
        (:`OnSuccess`
          (`KismetSystemLibrary.Delay` (`self.PatrolTime`))
          (`self.MoveToNextPatrol`))
        (:`OnFail`
          (`KismetSystemLibrary.Delay` 1.0)
          (`self.MoveToNextPatrol`))))))

(event `self.ReceiveTick`
  (params (DeltaSeconds :type "Float (single-precision)"))
  (`|ExecutionSequence`
    (:`then_0`
      (bind _aswd_enemy_life (cast `/Game/Blueprints/WD_EnemyLife` (`WidgetComponent.GetUserWidgetObject` (`self.Widget_Life`))))
      (`ProgressBar.SetPercent` (`/Game/Blueprints/WD_EnemyLife.EnemyLifeBar` _aswd_enemy_life) (/ (`self.CurrentLife`) 100.0)))
    (:`then_1`
      (bind _asbp_third_person_character (cast `/Game/ThirdPerson/Blueprints/BP_ThirdPersonCharacter` (`GameplayStatics.GetPlayerCharacter` 0)))
      (if (`/Game/ThirdPerson/Blueprints/BP_ThirdPersonCharacter.StoppGame` _asbp_third_person_character)
        (`self.NoFightMore`)))))

(fn `AttackEnemyStates`
  (params (CountDamage :type "Float (double-precision)"))
  (returns (EnemyState :type "/Game/Blueprints/EStatesEnemy Enum"))
  (`|ExecutionSequence`
    (:`then_0`
      (if (<= CountDamage 30.0)
        (bind _output_get (set `self.States` "NewEnumerator2"))
        (return _output_get)))
    (:`then_1`
      (if (<= CountDamage 60.0)
        (bind _output_get_2 (set `self.States` "NewEnumerator1"))
        (return _output_get_2)))
    (:`then_2`
      (if (<= CountDamage 100.0)
        (bind _output_get_3 (set `self.States` "NewEnumerator0"))
        (return _output_get_3)))))

(fn `GetDamage`
  (params (Damage :type "Float (double-precision)"))
  (returns (TotalDamage :type "Float (double-precision)"))
  (bind _output_get (set `self.CurrentLife` (`KismetMathLibrary.FClamp` (- (`self.CurrentLife`) Damage) 0.0 100.0)))
  (`|ExecutionSequence`
    (:`then_0`
      (`KismetSystemLibrary.PrintString` (`KismetStringLibrary.Conv_DoubleToString` _output_get))
      (if (== _output_get 0.0)
        (bind _asia_enemy (cast `/Game/IA_Animations/IA_Enemy` (`SkeletalMeshComponent.GetAnimInstance` (`self.Mesh`))))
        (set `/Game/IA_Animations/IA_Enemy.Death` true _asia_enemy)
        (set `/Game/IA_Animations/IA_Enemy.NoCollision` true _asia_enemy)
        (`PrimitiveComponent.SetCollisionEnabled` (`self.DamageRange`) "NoCollision")))
    (:`then_1`
      (return _output_get))))

(fn `UserConstructionScript`)