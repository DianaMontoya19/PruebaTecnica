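; Enemy AI pawn that chases the player and attacks at close range.
; Pawn sensing sets a detection flag, never cleared here, and issues an AI MoveTo toward the player character.
; Capsule overlap with the third-person character starts or stops a looping attack timer.
; Each attack raises the ExoAttack flag on the IA_Enemy anim instance, gated by range and a cooldown delay matching the timer interval.
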(event `self.PawnSensing.OnSeePawn`
  (params (Pawn :type "Pawn Object Reference"))
  (set `self.PlayerDetected` true)
  (`self.FollowPlayer`))

(event `FollowPlayer`
  (if (`self.PlayerDetected`)
    (`|AIMoveTo` self (0.0 0.0 0.0) (`GameplayStatics.GetPlayerCharacter` 0))))

(event `self.Capsule.OnComponentBeginOverlap`
  (params (OverlappedComponent :type "PrimitiveComponent Object Reference") (OtherActor :type "Actor Object Reference") (OtherComp :type "PrimitiveComponent Object Reference") (OtherBodyIndex :type Integer) (bFromSweep :type Boolean) (SweepResult :type "HitResult Structure (by ref)"))
  (cast `/Game/ThirdPerson/Blueprints/BP_ThirdPersonCharacter` OtherActor)
  (set `self.RangeOfAttack` true)
  (`self.StartAttackLoop`))

(event `self.Capsule.OnComponentEndOverlap`
  (params (OverlappedComponent :type "PrimitiveComponent Object Reference") (OtherActor :type "Actor Object Reference") (OtherComp :type "PrimitiveComponent Object Reference") (OtherBodyIndex :type Integer))
  (cast `/Game/ThirdPerson/Blueprints/BP_ThirdPersonCharacter` OtherActor)
  (set `self.RangeOfAttack` false)
  (`self.StopAttackLoop`))

(event `StartAttackLoop`
  (bind _returnvalue (`KismetSystemLibrary.K2_SetTimerDelegate` (delegate `PerfomAttack`) (`self.AttackCoolDown`) true))
  (set `self.LoopTimerAttack` _returnvalue))

(event `PerfomAttack`
  (if (`self.RangeOfAttack`)
    (if (`self.CanAttack`)
      (bind _asia_enemy (cast `/Game/IA_Animations/IA_Enemy` (`SkeletalMeshComponent.GetAnimInstance` (`self.Mesh`))))
      (set `/Game/IA_Animations/IA_Enemy.ExoAttack` true _asia_enemy)
      (set `self.CanAttack` false)
      (`KismetSystemLibrary.Delay` (`self.AttackCoolDown`))
      (set `self.CanAttack` true))))

(event `StopAttackLoop`
  (`KismetSystemLibrary.K2_ClearAndInvalidateTimerHandle` (`self.LoopTimerAttack`)))

(fn `UserConstructionScript`)